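; Save game object for the modular car system that stores a car build as its individual parts.
; SaveGame records each part's settings and actor transform, writing the part whose class is exactly BP_MasterCarPart to MasterPart and appending all others to NormalParts without clearing that array first.
; LoadGame only returns the stored master part and normal parts, with no spawning done here.
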(fn SaveGame
  (params (PartsToSave :type Array%20of%20BP%20Base%20Car%20Part%20Object%20References))
  (for _array_element PartsToSave
    (if (== (Utilities|GetClass _array_element) "/Game/ModularCarSystem/BluePrints/CarPart/BP_MasterCarPart.BP_MasterCarPart_C")
      (Utilities|Struct|SetmembersinST_CarSaveGameObject (Variables|Default|GetMasterPart) (Variables|/Game/ModularCarSystem/BluePrints/BP_BaseCarPart.BP_BaseCarPart_C|GetPart%20Settings _array_element) (Transformation|GetActorTransform _array_element))
      (else
        (Utilities|Array|Add (Variables|Default|GetNormalParts) (Utilities|Struct|MakeST_CarSaveGameObject (Variables|/Game/ModularCarSystem/BluePrints/BP_BaseCarPart.BP_BaseCarPart_C|GetPart%20Settings _array_element) (Transformation|GetActorTransform _array_element)))))))

(fn LoadGame
  (return (Variables|Default|GetMasterPart) (Variables|Default|GetNormalParts)))