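; Base player controller for the modular car system, handling player input and camera framing for building car parts.
; On BeginPlay it adds the Enhanced Input mapping context and registers itself with the BPCModularCar component.
; Input actions forward menu toggling, cancel, confirm, rotation and last-part placement to that component.
; An interface event plays a timeline that lerps the pawn's camera to an offset building view, or back to zero when reversed.
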(event EventBeginPlay
  (bind _self self)
  (bind _returnvalue (PlayerController|LocalPlayerSubsystems|GetEnhancedInputLocalPlayerSubsystem _self))
  ;[0.15 0.15 0.15 0.5] Start the input
  (Utilities|IsValid _returnvalue
    (:Is%20Valid
      (Input|AddMappingContext _returnvalue "/Game/ModularCarSystem/Inputs/IMC_ModularInputsDefault.IMC_ModularInputsDefault" 0 "(bIgnoreAllPressedKeysUntilRelease=True,bForceImmediately=False,bNotifyUserSettings=False)")
      (Variables|/Game/ModularCarSystem/Component/BPC_ModularCar.BPC_ModularCar_C|SetPlayerControllerRef (Variables|Default|GetBPCModularCar) self))))

(event EventTick
  (params (DeltaSeconds :type Float%20%28single-precision%29)))

(event Input|EnhancedActionEvents|EnhancedInputActionIA_ToggleBuildingPartsWidget
  (params (ActionValue :type Boolean) (ElapsedSeconds :type Float%20%28double-precision%29) (TriggeredSeconds :type Float%20%28double-precision%29) (InputAction :type Input%20Action%20Object%20Reference :default "/Game/ModularCarSystem/Inputs/ModularCar/IA_ToggleBuildingPartsWidget.IA_ToggleBuildingPartsWidget"))
  ;[0.15 0.15 0.15 0.5] Trigger the widget building menu
  (:Started
    (Default|APIToggleBuildingWidget (Variables|Default|GetBPCModularCar))))

(event Input|EnhancedActionEvents|EnhancedInputActionIA_CancelBuildingMode
  (params (ActionValue :type Boolean) (ElapsedSeconds :type Float%20%28double-precision%29) (TriggeredSeconds :type Float%20%28double-precision%29) (InputAction :type Input%20Action%20Object%20Reference :default "/Game/ModularCarSystem/Inputs/ModularCar/IA_CancelBuildingMode.IA_CancelBuildingMode"))
  ;[0.15 0.15 0.15 0.5] When the player cancel the building mode
  (:Started
    (Default|APICancelBuildingMode (Variables|Default|GetBPCModularCar))))

(event Input|EnhancedActionEvents|EnhancedInputActionIA_ConfirmBuildingMode
  (params (ActionValue :type Boolean) (ElapsedSeconds :type Float%20%28double-precision%29) (TriggeredSeconds :type Float%20%28double-precision%29) (InputAction :type Input%20Action%20Object%20Reference :default "/Game/ModularCarSystem/Inputs/ModularCar/IA_ConfirmBuildingMode.IA_ConfirmBuildingMode"))
  ;[0.15 0.15 0.15 0.5] Confirm part placement
  (:Started
    (Default|APIConfirmBuildingAction (Variables|Default|GetBPCModularCar))))

(event Input|EnhancedActionEvents|EnhancedInputActionIA_PartRotateUp
  (params (ActionValue :type Boolean) (ElapsedSeconds :type Float%20%28double-precision%29) (TriggeredSeconds :type Float%20%28double-precision%29) (InputAction :type Input%20Action%20Object%20Reference :default "/Game/ModularCarSystem/Inputs/ModularCar/IA_PartRotateUp.IA_PartRotateUp"))
  ;[0.15 0.15 0.15 0.5] Parts rotation
  (:Started
    (Default|APIRotatePart (Variables|Default|GetBPCModularCar) false)))

(event Input|EnhancedActionEvents|EnhancedInputActionIA_PartRotateDown
  (params (ActionValue :type Boolean) (ElapsedSeconds :type Float%20%28double-precision%29) (TriggeredSeconds :type Float%20%28double-precision%29) (InputAction :type Input%20Action%20Object%20Reference :default "/Game/ModularCarSystem/Inputs/ModularCar/IA_PartRotateDown.IA_PartRotateDown"))
  ;[0.15 0.15 0.15 0.5] Parts rotation
  (:Started
    (Default|APIRotatePart (Variables|Default|GetBPCModularCar) true)))

(event Input|EnhancedActionEvents|EnhancedInputActionIA_PlaceLastPart
  (params (ActionValue :type Boolean) (ElapsedSeconds :type Float%20%28double-precision%29) (TriggeredSeconds :type Float%20%28double-precision%29) (InputAction :type Input%20Action%20Object%20Reference :default "/Game/ModularCarSystem/Inputs/ModularCar/IA_PlaceLastPart.IA_PlaceLastPart"))
  ;[0.15 0.15 0.15 0.5] This will start the placement system with the last selected part
  (:Started
    (Default|APIOpenQuickPartPlace (Variables|Default|GetBPCModularCar))))

(event Custom|API_SetCameraModeBuildingSystem
  (params (isReverse :type Boolean))
  (bind _camera (Class|BPICharacterModularCar|IReturnCharacterCamera(Message) (Pawn|GetControlledPawn)))
  (bind _movecamera (Timeline|CameraMove PlayFromStart)
    (:Update
      (if (not isReverse)
        (CallFunction|APISetCameraLocation _camera "0.000000,80.000000,50.000000" _movecamera)
        (else
          (CallFunction|APISetCameraLocation _camera "0, 0, 0" _movecamera))))))

(event Custom|API_SetCameraLocation
  (params (Camera :type Scene%20Component%20Object%20Reference) (FinalLocation :type Vector) (Alpha :type Float%20%28single-precision%29))
  (Transformation|SetRelativeLocation Camera (Math|Vector|Lerp(Vector) (Variables|/Script/Engine.SceneComponent|GetRelativeLocation Camera) FinalLocation Alpha) false false))

(event EventITriggerPlayerCameraMode
  (params (isReverse :type Boolean))
  (CallFunction|APISetCameraModeBuildingSystem isReverse))

(fn ConstructionScript)