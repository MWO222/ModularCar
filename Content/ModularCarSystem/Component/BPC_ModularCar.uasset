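; Component that drives modular car building: choosing, placing, rotating and deleting parts, then possessing the car to test it.
; BeginPlay loads parts from a data table for the selection widget, and API events toggle widgets, input modes and build modes.
; Tick line-traces from the character camera to snap preview parts onto sockets or highlight deletion targets, applied on confirm.
; It also saves and loads car parts asynchronously in one fixed slot.
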(event EventBeginPlay
  ;[0.15 0.15 0.15 0.5] Get all parts for the widget
  (bind _outrownames (DataTable|GetDataTableRowNames "/Game/ModularCarSystem/Variables/PartsVariables/DT_BuildingCarParts.DT_BuildingCarParts"))
  (for _array_element _outrownames
    (bind _returnvalue (Utilities|GetDataTableRow "/Game/ModularCarSystem/Variables/PartsVariables/DT_BuildingCarParts.DT_BuildingCarParts" _array_element)
      (:then
        (Utilities|Array|Add (Variables|BuildingWidget|GetPartsWidget) _returnvalue)))))

(event EventTick
  (params (DeltaSeconds :type Float%20%28single-precision%29)))

(event Custom|API_ToggleBuildingWidget
  ;[0.0219 0.15 0.01596 0.5] Building list widget logic
  ;;[0.15 0.15 0.15 0.5] Toggle main widget
  (if (Variables|BuildingWidget|GetIsBuildingPartWidgetOpen)
    (CallFunction|APICloseBuildParts)
    (else
      (CallFunction|APIOpenBuildParts))))

(event Custom|API_SetGameMode
  ;[0.145 0.03637 0.15 0.5] Handle the game mode
  (Variables|/Script/Engine.PlayerController|SetbShowMouseCursor (Variables|Default|GetPlayerControllerRef) false)
  (Input|SetInputModeGameOnly (Variables|Default|GetPlayerControllerRef) false))

(event Custom|API_CarWidgetOpen
  ;[0 0.2848 0.2632] Car Widget Play info
  (Variables|CarWidget|SetCarInfoWidgetOpen true)
  (bind _returnvalue (UserInterface|CreateWidget "/Game/ModularCarSystem/Widget/CarInfoWidget/WBP_CarInfo.WBP_CarInfo_C" 0 self))
  (bind _output_get (Variables|Carwidget|SetCarWidgetRef _returnvalue))
  (UserInterface|Viewport|AddtoViewport _output_get 0)
  (CallFunction|APISetWidgetMode (Variables|Carwidget|GetCarWidgetRef)))

(event Custom|API_TogglePointWidget
  (bind _pointwidgetref (Variables|PointWidget|GetPointWidgetRef))
  ;[0.6573 0.6518 0.08943 0.5] Toggle the point vidget
  (if (not (Variables|PointWidget|GetIsPointWidgetOpen))
    (CallFunction|APIOpenPointWidget)
    (else
      (CallFunction|APIClosePointWidget)
      (Utilities|IsValid _pointwidgetref
        (:Is%20Valid
          (Widget|RemovefromParent _pointwidgetref)
          (Variables|PointWidget|SetIsPointWidgetOpen false))))))

(event Custom|API_ClosePointWidget
  (bind _pointwidgetref (Variables|PointWidget|GetPointWidgetRef))
  ;[0.6573 0.6518 0.08943 0.5] Toggle the point vidget
  (Utilities|IsValid _pointwidgetref
    (:Is%20Valid
      (Widget|RemovefromParent _pointwidgetref)
      (Variables|PointWidget|SetIsPointWidgetOpen false))))

(event Custom|API_SetWidgetMode
  (params (InWidgetToFocus :type Widget%20Object%20Reference))
  ;[0.145 0.03637 0.15 0.5] Handle the game mode
  (Variables|/Script/Engine.PlayerController|SetbShowMouseCursor (Variables|Default|GetPlayerControllerRef) true)
  (Input|SetInputModeGameandUI (Variables|Default|GetPlayerControllerRef) InWidgetToFocus "DoNotLock" true false))

(event Custom|API_OpenPointWidget
  ;[0.6573 0.6518 0.08943 0.5] Toggle the point vidget
  (bind _returnvalue (UserInterface|CreateWidget "/Game/ModularCarSystem/Widget/Target/WBP_TargetPoint.WBP_TargetPoint_C"))
  (bind _output_get (Variables|PointWidget|SetPointWidgetRef _returnvalue))
  (UserInterface|Viewport|AddtoViewport _output_get 0)
  (Variables|PointWidget|SetIsPointWidgetOpen true))

(event Custom|API_CloseBuildParts
  ;[0.0219 0.15 0.01596 0.5] Building list widget logic
  ;;[0.15 0.15 0.15 0.5] Handle the build parts widget
  (Variables|BuildingWidget|SetIsBuildingPartWidgetOpen false)
  (Utilities|IsValid (Variables|BuildingWidget|GetBuildingWidget)
    (:Is%20Valid
      (Widget|RemovefromParent (Variables|BuildingWidget|GetBuildingWidget)))
    (:Is%20Not%20Valid
      _))
  (CallFunction|APISetGameMode))

(event Custom|API_OpenBuildParts
  ;[0.0219 0.15 0.01596 0.5] Building list widget logic
  ;;[0.15 0.15 0.15 0.5] Handle the build parts widget
  (Variables|BuildingWidget|SetIsBuildingPartWidgetOpen true)
  (bind _returnvalue (UserInterface|CreateWidget "/Game/ModularCarSystem/Widget/ItemsList/WBP_ModularBuildSelection.WBP_ModularBuildSelection_C" 0 (Variables|BuildingWidget|GetPartsWidget) self))
  (bind _output_get (Variables|BuildingWidget|SetBuildingWidget _returnvalue))
  (UserInterface|Viewport|AddtoViewport _output_get 0)
  (CallFunction|APISetWidgetMode (Variables|BuildingWidget|GetBuildingWidget)))

(event Custom|API_ToogleCarInfoWidget
  (params (MasterCarPartRef :type BP%20Master%20Car%20Part%20Object%20Reference))
  ;[0 0.2848 0.2632] Car Widget Play info
  ;;[0.15 0.15 0.15 0.5] Toggle the car widget info
  (Utilities|IsValid MasterCarPartRef
    (:Is%20Valid
      (Variables|CarTesting|SetMaster%20Car%20Part%20Ref MasterCarPartRef))
    (:Is%20Not%20Valid
      _))
  (if (Variables|CarWidget|GetCarInfoWidgetOpen)
    (CallFunction|APICarWidgetClose)
    (else
      (CallFunction|APICarWidgetOpen))))

(event Custom|API_CarWidgetClose
  ;[0 0.2848 0.2632] Car Widget Play info
  (Variables|CarWidget|SetCarInfoWidgetOpen false)
  (Utilities|IsValid (Variables|Carwidget|GetCarWidgetRef)
    (:Is%20Valid
      (Widget|RemovefromParent (Variables|Carwidget|GetCarWidgetRef)))
    (:Is%20Not%20Valid
      _))
  (CallFunction|APISetGameMode))

(event Custom|API_StartBuildingCarMode
  (params (BuildingPartRef :type ST%20Car%20Parts%20Structure) (IsQuickAction :type Boolean))
  ;[0 0.6436 1 0.5] Start the building mode
  (Variables|BuildingMode|SetLastPlacedPart BuildingPartRef)
  (if (Utilities|Enum|Equal(Enum) (Variables|BuildingMode|GetBuildingSelectionMode) "NewEnumerator0")
    (CallFunction|APISpawnPreviewPart BuildingPartRef)
    (CallFunction|APITogglePointWidget)
    (if (not IsQuickAction)
      (CallFunction|APIToggleBuildingWidget))
    (Class|BPIModularCar|ITriggerPlayerCameraMode(Message) (Variables|Default|GetPlayerControllerRef) false)
    (Variables|BuildingMode|SetBuildingSelectionMode "NewEnumerator1")))

(event Custom|API_CancelBuildingMode
  (bind _deletemodehitactor (Variables|BuildingMode|GetDeleteModeHitActor))
  (bind _previewpart (Variables|BuildingMode|GetPreviewPart))
  ;[0.15 0.05068 0 0.5] Cancel the building mode
  (CallFunction|APIClosePointWidget)
  (Class|BPIModularCar|ITriggerPlayerCameraMode(Message) (Variables|Default|GetPlayerControllerRef) true)
  (Utilities|IsValid _deletemodehitactor
    (:Is%20Valid
      (Default|APIPartinPlacedMode _deletemodehitactor))
    (:Is%20Not%20Valid
      _))
  (Variables|BuildingMode|SetBuildingSelectionMode "NewEnumerator0")
  (Utilities|IsValid _previewpart
    (:Is%20Valid
      (Actor|DestroyActor _previewpart))))

(event Custom|API_SpawnPreviewPart
  (params (ST_CarParts :type ST%20Car%20Parts%20Structure%20%28by%20ref%29))
  (bind _playercontrollerref (Variables|Default|GetPlayerControllerRef))
  (bind _returnvalue (Pawn|GetControlledPawn _playercontrollerref))
  (bind _returnvalue_2 (Transformation|GetActorLocation _returnvalue))
  ;[0.3435 0.4029 1 0.5] Spawn the preview building part
  (bind _returnvalue_3 (Game|SpawnActorfromClass (Utilities|Struct|BreakST_CarParts ST_CarParts) (Math|Transform|MakeTransform (Math|Vector|MakeVector (.x _returnvalue_2) (.y _returnvalue_2) 8e+02)) "Undefined" "MultiplyWithRoot" 0 ST_CarParts 0))
  (bind _output_get (Variables|BuildingMode|SetPreviewPart _returnvalue_3))
  (Default|APIPartinPreviewMode _output_get))

(event Custom|API_ConfirmBuildingAction
  (bind _placementsocketref (Variables|BuildingMode|GetPlacementSocketRef))
  ;[0.005512 0.15 0.007526 0.5] Building confirm action
  (switch Utilities|FlowControl|Switch|SwitchonE_BuildingSelection (Variables|BuildingMode|GetBuildingSelectionMode)
    (:NewEnumerator1
      (if (Variables|BuildingMode|GetisPartPlacementAllowed)
        (Default|APIPartinPlacedMode (Variables|BuildingMode|GetPreviewPart) _placementsocketref)
        (Default|APIAddPartOrganizer (Variables|/Game/ModularCarSystem/BluePrints/Sockets/BP_BaseSocket.BP_BaseSocket_C|GetMasterPartRef _placementsocketref) (Variables|BuildingMode|GetPreviewPart))
        (Variables|BuildingMode|SetPreviewPart 0)
        (CallFunction|APICancelBuildingMode)))
    (:NewEnumerator2
      (CallFunction|APICancelBuildingMode)
      (Actor|DestroyActor (Variables|BuildingMode|GetDeleteModeHitActor)))))

(event Custom|API_RotatePart
  (params (IsReverse :type Boolean))
  ;[0 0.8248 0.5454] Rotate Part
  (Utilities|IsValid (Variables|BuildingMode|GetPreviewPart)
    (:Is%20Valid
      (if IsReverse
        (CallFunction|APIPartRotation "0.000000,-90.000000,0.000000")
        (else
          (CallFunction|APIPartRotation "0.000000,90.000000,0.000000"))))))

(event Custom|API_PartRotation
  (params (NewRotation :type Rotator))
  (bind _previewpart (Variables|BuildingMode|GetPreviewPart))
  ;[0 0.8248 0.5454] Rotate Part
  (Transformation|SetActorRotation _previewpart (Math|Rotator|CombineRotators (Transformation|GetActorRotation _previewpart) NewRotation)))

(event Custom|API_OpenQuickPartPlace
  ;[0.9905 1 0.09107 0.5] Quick action
  (if (Utilities|IsValidClass (.PartClass (Utilities|Struct|BreakST_CarParts (Variables|BuildingMode|GetLastPlacedPart))))
    (CallFunction|APIStartBuildingCarMode (Variables|BuildingMode|GetLastPlacedPart) true)))

(event Custom|API_DeleteMode
  ;[1 0.06202 0.1589] Delete mode
  (Class|BPIModularCar|ITriggerPlayerCameraMode(Message) (Variables|Default|GetPlayerControllerRef) false)
  (Variables|BuildingMode|SetBuildingSelectionMode "NewEnumerator2")
  (CallFunction|APITogglePointWidget)
  (CallFunction|APIToggleBuildingWidget))

(event EventTick
  (params (DeltaSeconds :type Float%20%28single-precision%29))
  (bind _previewpart (Variables|BuildingMode|GetPreviewPart))
  (switch Utilities|FlowControl|Switch|SwitchonE_BuildingSelection (Variables|BuildingMode|GetBuildingSelectionMode)
    (:NewEnumerator1
      ;[0.15 0.15 0.15 0.5] Part Placement
      (bind (_outhit _validhit) (CallFunction|HandleCameraLineTrace))
      (if _validhit
        (Utilities|IsValid _previewpart
          (:Is%20Valid
            (if (not (== (Utilities|GetClass (.HitActor (Collision|BreakHitResult _outhit))) "/Game/ModularCarSystem/BluePrints/Sockets/BP_BaseSocket.BP_BaseSocket_C"))
              (Transformation|SetActorLocation _previewpart (.Location (Collision|BreakHitResult _outhit)) false false)
              (Default|APIPreviewModeNotAllowed _previewpart)
              (Variables|BuildingMode|SetisPartPlacementAllowed false)
              (else
                (bind _socket (Class|BPIBaseSocket|IReturnSocketRef(Message) (.HitActor (Collision|BreakHitResult _outhit))))
                (bind _output_get (Variables|BuildingMode|SetPlacementSocketRef _socket))
                (bind _locationoffset (Default|GetPartOffset _output_get (Variables|BuildingMode|GetPreviewPart)))
                (Transformation|SetActorLocation (Variables|BuildingMode|GetPreviewPart) (+ (Transformation|GetActorLocation (.HitActor (Collision|BreakHitResult _outhit))) _locationoffset) false false)
                (Default|APIPartinPreviewMode (Variables|BuildingMode|GetPreviewPart))
                (Variables|BuildingMode|SetisPartPlacementAllowed true)))))))
    (:NewEnumerator2
      (bind (_outhit_2 _validhit_2) (CallFunction|HandleCameraLineTrace))
      (if _validhit_2
        (if (== (Utilities|GetClass (.HitActor (Collision|BreakHitResult _outhit_2))) "/Game/ModularCarSystem/BluePrints/Sockets/BP_BaseSocket.BP_BaseSocket_C")
          (bind _socket_2 (Class|BPIBaseSocket|IReturnSocketRef(Message) (.HitActor (Collision|BreakHitResult _outhit_2))))
          (CallFunction|HandleDeletePartSelect _socket_2 (Variables|/Game/ModularCarSystem/BluePrints/Sockets/BP_BaseSocket.BP_BaseSocket_C|GetAttachedActor _socket_2))
          (else
            (bind _asbp_base_car_part (Utilities|Casting|CastToBP_BaseCarPart (.HitActor (Collision|BreakHitResult _outhit_2))))
            (if (and (== _asbp_base_car_part (Variables|BuildingMode|GetDeleteModeHitActor)) (Utilities|IsValid (Variables|BuildingMode|GetDeleteModeHitActor)))
              (Default|APIPreviewModeNotAllowed (Variables|BuildingMode|GetDeleteModeHitActor))
              (else
                (Utilities|IsValid (Variables|BuildingMode|GetDeleteModeHitActor)
                  (:Is%20Valid
                    (Default|APIPartinPlacedMode (Variables|BuildingMode|GetDeleteModeHitActor)))
                  (:Is%20Not%20Valid
                    _))
                (bind _output_get_2 (Variables|BuildingMode|SetDeleteModeHitActor _asbp_base_car_part))
                (Default|APIPreviewModeNotAllowed _output_get_2)))))))))

(event Custom|API_TestModularCar
  (bind _master_car_part_ref (Variables|CarTesting|GetMaster%20Car%20Part%20Ref))
  (Default|APISimulate _master_car_part_ref)
  (CallFunction|APIToogleCarInfoWidget)
  (Pawn|Possess (Variables|Default|GetPlayerControllerRef) _master_car_part_ref))

(event Custom|API_SaveGame
  (bind _returnvalue (SaveGame|CreateSaveGameObject "/Game/ModularCarSystem/SaveGame/BP_modularCarSaveGame.BP_modularCarSaveGame_C"))
  (bind _outactors (Actor|GetAllActorsOfClass "/Game/ModularCarSystem/BluePrints/BP_BaseCarPart.BP_BaseCarPart_C"))
  (Default|SaveGame _returnvalue _outactors)
  (|AsyncSaveGametoSlot _returnvalue "Car01"
    (:Completed
      (Development|PrintString "Saved" true true "(R=0.274801,G=1.000000,B=0.000000,A=1.000000)"))))

(event Custom|API_LoadGame
  (bind _savegame (|AsyncLoadGamefromSlot "Car01")
    (:Completed
      (bind _asbp_modular_car_save_game (Utilities|Casting|CastToBP_modularCarSaveGame _savegame))
      (Default|LoadGame _asbp_modular_car_save_game))))

(fn HandleCameraLineTrace
  (bind _camera (Class|BPICharacterModularCar|IReturnCharacterCamera(Message) (Pawn|GetControlledPawn (Variables|Default|GetPlayerControllerRef))))
  (bind (_outhit _returnvalue) (Collision|LineTraceByChannel (Transformation|GetWorldLocation _camera) (+ (Transformation|GetWorldLocation _camera) (* (Math|Vector|GetForwardVector (Transformation|GetWorldRotation _camera)) 1.5e+03)) "TraceTypeQuery1" false 0 "ForOneFrame"))
  (return _outhit _returnvalue))

(fn HandleDeletePartSelect
  (params (NewActor :type BP%20Base%20Socket%20Object%20Reference) (CheckActor :type BP%20Base%20Car%20Part%20Object%20Reference))
  (if (and (== CheckActor (Variables|BuildingMode|GetDeleteModeHitActor)) (Utilities|IsValid (Variables|BuildingMode|GetDeleteModeHitActor)))
    (Default|APIPreviewModeNotAllowed (Variables|BuildingMode|GetDeleteModeHitActor))
    (else
      (Utilities|IsValid (Variables|BuildingMode|GetDeleteModeHitActor)
        (:Is%20Valid
          (Default|APIPartinPlacedMode (Variables|BuildingMode|GetDeleteModeHitActor) NewActor))
        (:Is%20Not%20Valid
          _))
      (bind _output_get (Variables|BuildingMode|SetDeleteModeHitActor CheckActor))
      (Default|APIPreviewModeNotAllowed _output_get))))