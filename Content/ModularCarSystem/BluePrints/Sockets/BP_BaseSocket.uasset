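; BP_BaseSocket is the base socket actor of the modular car system, with a sphere component that it hides on BeginPlay.
; API_SocketSetMasterPart stores a master part reference and records it as the attached actor.
; GetPartOffset maps a part's category to a local offset, lowering front and back wheels while other categories stay at zero.
; An interface-style function, IReturnSocketRef, returns the socket itself.
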(event Custom|API_SocketSetMasterPart
  (params (MasterPartRef :type BP%20Master%20Car%20Part%20Object%20Reference))
  ;[0.15 0.15 0.15 0.5] API Set master Part
  (Variables|Default|SetMasterPartRef MasterPartRef)
  (Variables|Default|SetAttachedActor MasterPartRef))

(event EventBeginPlay
  (Rendering|SetVisibility (Variables|Default|GetSphere) false false))

(event Collision|EventActorBeginOverlap
  (params (OtherActor :type Actor%20Object%20Reference)))

(event EventTick
  (params (DeltaSeconds :type Float%20%28single-precision%29)))

(fn ConstructionScript)

(fn GetPartOffset
  (params (Part :type BP%20Base%20Car%20Part%20Object%20Reference))
  (switch Utilities|FlowControl|Switch|SwitchonE_PartCategory (.Category (Utilities|Struct|BreakST_CarParts (Variables|/Game/ModularCarSystem/BluePrints/BP_BaseCarPart.BP_BaseCarPart_C|GetPart%20Settings Part)))
    (:NewEnumerator0
      (LocalVariables|SetOffset "0, 0, 0"))
    (:NewEnumerator1
      (LocalVariables|SetOffset "0.000000,0.000000,-38.000000"))
    (:NewEnumerator2
      (LocalVariables|SetOffset "0.000000,0.000000,-38.000000"))
    (:NewEnumerator3
      (LocalVariables|SetOffset "0, 0, 0"))
    (:NewEnumerator4
      (LocalVariables|SetOffset "0, 0, 0")))
  (return (LocalVariables|GetOffset)))

(fn IReturnSocketRef
  (return self))