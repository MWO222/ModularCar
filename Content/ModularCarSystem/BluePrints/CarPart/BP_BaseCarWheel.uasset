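; Base wheel part for the modular car system, with a placement preview state and a physics-driven active state.
; Preview mode makes the wheel ignore Visibility, Camera and Pawn channels and applies the placement-allowed material; placed mode restores blocking and the material cached at BeginPlay.
; Starting the wheel links it to a given body component through suspension and axis physics constraints, then enables physics simulation.
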(event Custom|API_SetConstrainBone
  (params (TargetUpdate :type Physics%20Constraint%20Component%20Object%20Reference) (WheelComponent :type Primitive%20Component%20Object%20Reference) (BodyComponent :type Primitive%20Component%20Object%20Reference))
  ;[0.15 0.15 0.15 0.5] Activate wheel logic
  (Class|PhysicsConstraintComponent|SetConstrainedComponents TargetUpdate WheelComponent "None" BodyComponent "None"))

(event Custom|API_StartWheel
  (params (BodyComponent :type Primitive%20Component%20Object%20Reference))
  ;[0.15 0.15 0.15 0.5] Activate wheel logic
  (CallFunction|APISetConstrainBone (Variables|Default|GetPC_WheelSuspension) (Variables|Default|GetWheel) BodyComponent)
  (CallFunction|APISetConstrainBone (Variables|Default|GetPC_WheelAxis) (Variables|Default|GetWheel) BodyComponent)
  (Physics|SetSimulatePhysics (Variables|Default|GetWheel) true))

(event EventBeginPlay
  (Variables|Default|SetOriginalMaterial (Rendering|Material|GetMaterial (Variables|Default|GetWheel) 0)))

(event Collision|EventActorBeginOverlap
  (params (OtherActor :type Actor%20Object%20Reference)))

(event EventTick
  (params (DeltaSeconds :type Float%20%28single-precision%29)))

(fn ConstructionScript
  (|CallParentFunction))

(fn InPreviewMode
  (bind _wheel (Variables|Default|GetWheel))
  (|CallParentFunction)
  (Collision|SetCollisionResponsetoChannel _wheel "ECC_Visibility" "ECR_Ignore")
  (Collision|SetCollisionResponsetoChannel _wheel "ECC_Camera" "ECR_Ignore")
  (Collision|SetCollisionResponsetoChannel _wheel "ECC_Pawn" "ECR_Ignore")
  (Rendering|Material|SetMaterial (Variables|Default|GetWheel) 0 (Variables|Default|GetPreviewMaterialPlaceAllowed)))

(fn PlacedMode
  (bind _wheel (Variables|Default|GetWheel))
  (|CallParentFunction)
  (Collision|SetCollisionResponsetoChannel _wheel "ECC_Visibility" "ECR_Block")
  (Collision|SetCollisionResponsetoChannel _wheel "ECC_Camera" "ECR_Block")
  (Collision|SetCollisionResponsetoChannel _wheel "ECC_Pawn" "ECR_Block")
  (Rendering|Material|SetMaterial (Variables|Default|GetWheel) 0 (Variables|Default|GetOriginalMaterial)))