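; Base wheel part for the modular car system, handling placement preview and physical attachment to the car body.
; Preview states swap the wheel's material to show whether placement is allowed, with collision disabled on entering preview.
; Placing restores collision and the original material, then, given a valid socket, binds the wheel to the master part's body through suspension and axis physics constraints and enables physics simulation.
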(event Custom|API_SetConstrainBone
  (params (TargetUpdate :type Physics%20Constraint%20Component%20Object%20Reference) (WheelComponent :type Primitive%20Component%20Object%20Reference) (BodyComponent :type Primitive%20Component%20Object%20Reference))
  ;[0.15 0.15 0.15 0.5] Activate wheel logic
  (Class|PhysicsConstraintComponent|SetConstrainedComponents TargetUpdate WheelComponent "None" BodyComponent "None"))

(event Custom|API_StartWheel
  (params (BodyComponent :type Primitive%20Component%20Object%20Reference))
  ;[0.15 0.15 0.15 0.5] Activate wheel logic
  (CallFunction|APISetConstrainBone (Variables|Default|GetPC_WheelSuspension) (Variables|Default|GetWheel) BodyComponent)
  (CallFunction|APISetConstrainBone (Variables|Default|GetPC_WheelAxis) (Variables|Default|GetWheel) BodyComponent)
  (Physics|SetSimulatePhysics (Variables|Default|GetWheel) true))

(event EventBeginPlay
  (Variables|Default|SetOriginalMaterial (Rendering|Material|GetMaterial (Variables|Default|GetWheel) 0)))

(event Collision|EventActorBeginOverlap
  (params (OtherActor :type Actor%20Object%20Reference)))

(event EventTick
  (params (DeltaSeconds :type Float%20%28single-precision%29)))

(fn ConstructionScript
  (|CallParentFunction))

(fn InPreviewMode
  (|CallParentFunction)
  (CallFunction|APIDisablePartCollision (Variables|Default|GetWheel))
  (Rendering|Material|SetMaterial (Variables|Default|GetWheel) 0 (Variables|Default|GetPreviewMaterialPlaceAllowed)))

(fn PlacedMode
  (params (SocketRef :type BP%20Base%20Socket%20Object%20Reference))
  (|CallParentFunction 0)
  (CallFunction|APIEnablePartCollision (Variables|Default|GetWheel))
  (Rendering|Material|SetMaterial (Variables|Default|GetWheel) 0 (Variables|Default|GetOriginalMaterial))
  (Utilities|IsValid SocketRef
    (:Is%20Valid
      (CallFunction|APIStartWheel (Variables|/Game/ModularCarSystem/BluePrints/CarPart/BP_MasterCarPart.BP_MasterCarPart_C|GetBody (Variables|/Game/ModularCarSystem/BluePrints/Sockets/BP_BaseSocket.BP_BaseSocket_C|GetMasterPartRef SocketRef))))))

(fn PartSimulate
  (|CallParentFunction)
  (Physics|SetSimulatePhysics (Variables|Default|GetWheel) true))

(fn PreviewModeNotAllowed
  (|CallParentFunction)
  (Rendering|Material|SetMaterial (Variables|Default|GetWheel) 0 (Variables|Default|GetPreviewMaterialPlaceNotAllowed)))

(fn IReturnPartReference
  (return 0))