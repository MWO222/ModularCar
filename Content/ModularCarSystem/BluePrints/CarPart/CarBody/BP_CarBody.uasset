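; BP_CarBody is the car body part of a modular car system, with six sockets and preview and placed states.
; Preview disables body and socket collision and swaps in an allowed or not-allowed placement material.
; Placing restores collision and the material cached at BeginPlay.
; Given a valid socket, it passes that socket's master part to its own sockets and attaches Body to the master's Body, keeping world transform.
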(event EventBeginPlay
  (|CallParentFunction)
  (Variables|Default|SetOriginalMaterial (Rendering|Material|GetMaterial (Variables|Default|GetBody) 0)))

(event Collision|EventActorBeginOverlap
  (params (OtherActor :type Actor%20Object%20Reference))
  (|CallParentFunction OtherActor) ; This node is disabled and will not be called.\nDrag off pins to build functionality.
)

(event EventTick
  (params (DeltaSeconds :type Float%20%28single-precision%29))
  (|CallParentFunction DeltaSeconds))

(fn ConstructionScript
  (|CallParentFunction))

(fn InPreviewMode
  (|CallParentFunction)
  (CallFunction|APIDisablePartCollision (Variables|Default|GetBody))
  (Rendering|Material|SetMaterial (Variables|Default|GetBody) 0 (Variables|Default|GetPreviewMaterialPlaceAllowed))
  (CallFunction|APIDisableSocketCollision (Variables|Default|GetSocket01))
  (CallFunction|APIDisableSocketCollision (Variables|Default|GetSocket02))
  (CallFunction|APIDisableSocketCollision (Variables|Default|GetSocket03))
  (CallFunction|APIDisableSocketCollision (Variables|Default|GetSocket04))
  (CallFunction|APIDisableSocketCollision (Variables|Default|GetSocket05))
  (CallFunction|APIDisableSocketCollision (Variables|Default|GetSocket06)))

(fn PlacedMode
  (params (SocketRef :type BP%20Base%20Socket%20Object%20Reference))
  (bind _output_get (LocalVariables|SetExternalPlacedSocketRef SocketRef))
  (|CallParentFunction _output_get)
  (CallFunction|APIEnablePartCollision (Variables|Default|GetBody))
  (Rendering|Material|SetMaterial (Variables|Default|GetBody) 0 (Variables|Default|GetOriginalMaterial))
  ;[0.15 0.15 0.15 0.5] Sockets enable handle
  (CallFunction|APIEnableSocketCollision (Variables|Default|GetSocket01))
  (CallFunction|APIEnableSocketCollision (Variables|Default|GetSocket02))
  (CallFunction|APIEnableSocketCollision (Variables|Default|GetSocket03))
  (CallFunction|APIEnableSocketCollision (Variables|Default|GetSocket04))
  (CallFunction|APIEnableSocketCollision (Variables|Default|GetSocket05))
  (CallFunction|APIEnableSocketCollision (Variables|Default|GetSocket06))
  (Utilities|IsValid (LocalVariables|GetExternalPlacedSocketRef)
    (:Is%20Valid
      ;[0.15 0.15 0.15 0.5] For the sockets we are passing the master part as a reference
      (CallFunction|APISetSocketMasterPartRef (Variables|Default|GetSocket01) (Variables|/Game/ModularCarSystem/BluePrints/Sockets/BP_BaseSocket.BP_BaseSocket_C|GetMasterPartRef (LocalVariables|GetExternalPlacedSocketRef)))
      (CallFunction|APISetSocketMasterPartRef (Variables|Default|GetSocket02) (Variables|/Game/ModularCarSystem/BluePrints/Sockets/BP_BaseSocket.BP_BaseSocket_C|GetMasterPartRef (LocalVariables|GetExternalPlacedSocketRef)))
      (CallFunction|APISetSocketMasterPartRef (Variables|Default|GetSocket03) (Variables|/Game/ModularCarSystem/BluePrints/Sockets/BP_BaseSocket.BP_BaseSocket_C|GetMasterPartRef (LocalVariables|GetExternalPlacedSocketRef)))
      (CallFunction|APISetSocketMasterPartRef (Variables|Default|GetSocket04) (Variables|/Game/ModularCarSystem/BluePrints/Sockets/BP_BaseSocket.BP_BaseSocket_C|GetMasterPartRef (LocalVariables|GetExternalPlacedSocketRef)))
      (CallFunction|APISetSocketMasterPartRef (Variables|Default|GetSocket05) (Variables|/Game/ModularCarSystem/BluePrints/Sockets/BP_BaseSocket.BP_BaseSocket_C|GetMasterPartRef (LocalVariables|GetExternalPlacedSocketRef)))
      (CallFunction|APISetSocketMasterPartRef (Variables|Default|GetSocket06) (Variables|/Game/ModularCarSystem/BluePrints/Sockets/BP_BaseSocket.BP_BaseSocket_C|GetMasterPartRef (LocalVariables|GetExternalPlacedSocketRef)))
      (Transformation|AttachComponentToComponent (Variables|Default|GetBody) (Variables|/Game/ModularCarSystem/BluePrints/CarPart/BP_MasterCarPart.BP_MasterCarPart_C|GetBody (Variables|/Game/ModularCarSystem/BluePrints/Sockets/BP_BaseSocket.BP_BaseSocket_C|GetMasterPartRef (LocalVariables|GetExternalPlacedSocketRef))) "None" "KeepWorld" "KeepWorld" "KeepWorld" true))))

(fn IReturnPartReference
  (return 0))

(fn PreviewModeNotAllowed
  (|CallParentFunction)
  (Rendering|Material|SetMaterial (Variables|Default|GetBody) 0 (Variables|Default|GetPreviewMaterialPlaceNotAllowed)))

(fn PartSimulate
  (|CallParentFunction))