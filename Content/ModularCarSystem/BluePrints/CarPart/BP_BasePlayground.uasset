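; BP_BasePlayground is a modular car system actor that initializes four wheels on a body.
; On BeginPlay it casts the child actors of Wheel01 through Wheel04 to BP_BaseCarWheel in sequence and calls APIStartWheel on each, passing Body.
; The casts are chained, so a failed cast leaves that wheel and all later ones uninitialized.
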(event Collision|EventActorBeginOverlap
  (params (OtherActor :type Actor%20Object%20Reference)))

(event EventBeginPlay
  (bind _asbp_base_car_wheel (Utilities|Casting|CastToBP_BaseCarWheel (Variables|/Script/Engine.ChildActorComponent|GetChildActor (Variables|Default|GetWheel01))))
  (Default|APIStartWheel _asbp_base_car_wheel (Variables|Default|GetBody))
  (bind _asbp_base_car_wheel_2 (Utilities|Casting|CastToBP_BaseCarWheel (Variables|/Script/Engine.ChildActorComponent|GetChildActor (Variables|Default|GetWheel02))))
  (Default|APIStartWheel _asbp_base_car_wheel_2 (Variables|Default|GetBody))
  (bind _asbp_base_car_wheel_3 (Utilities|Casting|CastToBP_BaseCarWheel (Variables|/Script/Engine.ChildActorComponent|GetChildActor (Variables|Default|GetWheel03))))
  (Default|APIStartWheel _asbp_base_car_wheel_3 (Variables|Default|GetBody))
  (bind _asbp_base_car_wheel_4 (Utilities|Casting|CastToBP_BaseCarWheel (Variables|/Script/Engine.ChildActorComponent|GetChildActor (Variables|Default|GetWheel04))))
  (Default|APIStartWheel _asbp_base_car_wheel_4 (Variables|Default|GetBody)))

(fn ConstructionScript)