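; Base car body part for the modular car system, with separate preview and placed states.
; On BeginPlay it caches the Body mesh's first material as the original.
; Preview mode makes the body ignore the Visibility, Camera and Pawn channels and applies the preview material.
; Placed mode sets those channels back to Block and restores the original material, with both modes extending the parent class's logic.
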(event EventBeginPlay
  (|CallParentFunction)
  (Variables|Default|SetOriginalMaterial (Rendering|Material|GetMaterial (Variables|Default|GetBody) 0)))

(event Collision|EventActorBeginOverlap
  (params (OtherActor :type Actor%20Object%20Reference))
  (|CallParentFunction OtherActor) ; This node is disabled and will not be called.\nDrag off pins to build functionality.
)

(event EventTick
  (params (DeltaSeconds :type Float%20%28single-precision%29))
  (|CallParentFunction DeltaSeconds))

(fn ConstructionScript
  (|CallParentFunction))

(fn InPreviewMode
  (bind _body (Variables|Default|GetBody))
  (|CallParentFunction)
  (Collision|SetCollisionResponsetoChannel _body "ECC_Visibility" "ECR_Ignore")
  (Collision|SetCollisionResponsetoChannel _body "ECC_Camera" "ECR_Ignore")
  (Collision|SetCollisionResponsetoChannel _body "ECC_Pawn" "ECR_Ignore")
  (Rendering|Material|SetMaterial (Variables|Default|GetBody) 0 (Variables|Default|GetPreviewMaterial)))

(fn PlacedMode
  (bind _body (Variables|Default|GetBody))
  (|CallParentFunction)
  (Collision|SetCollisionResponsetoChannel _body "ECC_Visibility" "ECR_Block")
  (Collision|SetCollisionResponsetoChannel _body "ECC_Camera" "ECR_Block")
  (Collision|SetCollisionResponsetoChannel _body "ECC_Pawn" "ECR_Block")
  (Rendering|Material|SetMaterial (Variables|Default|GetBody) 0 (Variables|Default|GetOriginalMaterial)))