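; Root part of the modular car system, the body that other parts attach to through six sockets.
; On BeginPlay it registers itself as master on each socket and sorts reported parts into body and front-wheel lists.
; Preview and placed modes toggle body and socket collision and swap materials to show placement validity.
; Simulate enables physics on itself and simulates body parts, while the front-wheel loop's simulate call is left unwired.
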(event Custom|API_Simulate
  ;[0.15 0.15 0.15 0.5] This will simulate the car
  (CallFunction|APIPartSimulate)
  (for _array_element (Variables|Part|GetBodyParts)
    (Default|APIPartSimulate _array_element))
  (for _array_element_2 (Variables|Part|GetFrontWheelParts)
    _))

(event Custom|API_AddPartOrganizer
  (params (ModularPart :type BP%20Base%20Car%20Part%20Object%20Reference))
  ;[0.6156 0 0.5282] Add unique parts to the organizer
  (switch Utilities|FlowControl|Switch|SwitchonE_PartCategory (.Category (Utilities|Struct|BreakST_CarParts (Variables|/Game/ModularCarSystem/BluePrints/BP_BaseCarPart.BP_BaseCarPart_C|GetPart%20Settings ModularPart)))
    (:NewEnumerator0
      (Utilities|Array|AddUnique (Variables|Part|GetBodyParts) ModularPart))
    (:NewEnumerator2
      (Utilities|Array|AddUnique (Variables|Part|GetFrontWheelParts) ModularPart))))

(event EventBeginPlay
  (|CallParentFunction)
  (Variables|Default|SetOriginalMaterial (Rendering|Material|GetMaterial (Variables|Default|GetBody) 0))
  ;[0.15 0.15 0.15 0.5] Start the reference of the master part in the socket
  (CallFunction|APISetSocketMasterPartRef (Variables|Default|GetSocket01) self)
  (CallFunction|APISetSocketMasterPartRef (Variables|Default|GetSocket02) self)
  (CallFunction|APISetSocketMasterPartRef (Variables|Default|GetSocket03) self)
  (CallFunction|APISetSocketMasterPartRef (Variables|Default|GetSocket04) self)
  (CallFunction|APISetSocketMasterPartRef (Variables|Default|GetSocket05) self)
  (CallFunction|APISetSocketMasterPartRef (Variables|Default|GetSocket06) self))

(event Collision|EventActorBeginOverlap
  (params (OtherActor :type Actor%20Object%20Reference))
  (|CallParentFunction OtherActor) ; This node is disabled and will not be called.\nDrag off pins to build functionality.
)

(event EventTick
  (params (DeltaSeconds :type Float%20%28single-precision%29))
  (|CallParentFunction DeltaSeconds))

(fn ConstructionScript
  (|CallParentFunction))

(fn InPreviewMode
  (|CallParentFunction)
  (CallFunction|APIDisablePartCollision (Variables|Default|GetBody))
  (Rendering|Material|SetMaterial (Variables|Default|GetBody) 0 (Variables|Default|GetPreviewMaterialPlaceAllowed))
  (CallFunction|APIDisableSocketCollision (Variables|Default|GetSocket01))
  (CallFunction|APIDisableSocketCollision (Variables|Default|GetSocket02))
  (CallFunction|APIDisableSocketCollision (Variables|Default|GetSocket03))
  (CallFunction|APIDisableSocketCollision (Variables|Default|GetSocket04))
  (CallFunction|APIDisableSocketCollision (Variables|Default|GetSocket05))
  (CallFunction|APIDisableSocketCollision (Variables|Default|GetSocket06)))

(fn PlacedMode
  (params (SocketRef :type BP%20Base%20Socket%20Object%20Reference))
  (|CallParentFunction 0)
  (CallFunction|APIEnablePartCollision (Variables|Default|GetBody))
  (Rendering|Material|SetMaterial (Variables|Default|GetBody) 0 (Variables|Default|GetOriginalMaterial))
  ;[0.15 0.15 0.15 0.5] Sockets enable handle
  (CallFunction|APIEnableSocketCollision (Variables|Default|GetSocket01))
  (CallFunction|APIEnableSocketCollision (Variables|Default|GetSocket02))
  (CallFunction|APIEnableSocketCollision (Variables|Default|GetSocket03))
  (CallFunction|APIEnableSocketCollision (Variables|Default|GetSocket04))
  (CallFunction|APIEnableSocketCollision (Variables|Default|GetSocket05))
  (CallFunction|APIEnableSocketCollision (Variables|Default|GetSocket06)))

(fn IReturnPartReference
  (return 0))

(fn PreviewModeNotAllowed
  (|CallParentFunction)
  (Rendering|Material|SetMaterial (Variables|Default|GetBody) 0 (Variables|Default|GetPreviewMaterialPlaceNotAllowed)))

(fn PartSimulate
  (|CallParentFunction)
  (Physics|SetSimulatePhysics (Variables|Default|GetBody) true))