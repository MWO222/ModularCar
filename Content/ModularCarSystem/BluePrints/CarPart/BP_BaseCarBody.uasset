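; Base car body part for a modular car system, with six child-actor sockets and preview and placed states.
; It caches the body's original material on BeginPlay.
; Preview mode swaps in a preview material and ignores Visibility, Camera and Pawn collision on the body and only the first socket's sphere.
; Placed mode restores the material and enables collision on the body and all six sockets.
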(event EventBeginPlay
  (|CallParentFunction)
  (Variables|Default|SetOriginalMaterial (Rendering|Material|GetMaterial (Variables|Default|GetBody) 0)))

(event Collision|EventActorBeginOverlap
  (params (OtherActor :type Actor%20Object%20Reference))
  (|CallParentFunction OtherActor) ; This node is disabled and will not be called.\nDrag off pins to build functionality.
)

(event EventTick
  (params (DeltaSeconds :type Float%20%28single-precision%29))
  (|CallParentFunction DeltaSeconds))

(fn ConstructionScript
  (|CallParentFunction))

(fn InPreviewMode
  (bind _body (Variables|Default|GetBody))
  (|CallParentFunction)
  (Collision|SetCollisionResponsetoChannel _body "ECC_Visibility" "ECR_Ignore")
  (Collision|SetCollisionResponsetoChannel _body "ECC_Camera" "ECR_Ignore")
  (Collision|SetCollisionResponsetoChannel _body "ECC_Pawn" "ECR_Ignore")
  (Rendering|Material|SetMaterial (Variables|Default|GetBody) 0 (Variables|Default|GetPreviewMaterial))
  (bind _asbp_base_socket (Utilities|Casting|CastToBP_BaseSocket (Variables|/Script/Engine.ChildActorComponent|GetChildActor (Variables|Default|GetSocket01))))
  (Collision|SetCollisionResponsetoChannel (Variables|/Game/ModularCarSystem/BluePrints/Sockets/BP_BaseSocket.BP_BaseSocket_C|GetSphere _asbp_base_socket) "ECC_Visibility" "ECR_Ignore")
  (Collision|SetCollisionResponsetoChannel (Variables|/Game/ModularCarSystem/BluePrints/Sockets/BP_BaseSocket.BP_BaseSocket_C|GetSphere _asbp_base_socket) "ECC_Camera" "ECR_Ignore")
  (Collision|SetCollisionResponsetoChannel (Variables|/Game/ModularCarSystem/BluePrints/Sockets/BP_BaseSocket.BP_BaseSocket_C|GetSphere _asbp_base_socket) "ECC_Pawn" "ECR_Ignore"))

(fn PlacedMode
  (|CallParentFunction)
  (CallFunction|APIEnablePartCollision (Variables|Default|GetBody))
  (Rendering|Material|SetMaterial (Variables|Default|GetBody) 0 (Variables|Default|GetOriginalMaterial))
  ;[0.15 0.15 0.15 0.5] Sockets enable handle
  (CallFunction|APIEnableSocketCollision (Variables|Default|GetSocket01))
  (CallFunction|APIEnableSocketCollision (Variables|Default|GetSocket02))
  (CallFunction|APIEnableSocketCollision (Variables|Default|GetSocket03))
  (CallFunction|APIEnableSocketCollision (Variables|Default|GetSocket04))
  (CallFunction|APIEnableSocketCollision (Variables|Default|GetSocket05))
  (CallFunction|APIEnableSocketCollision (Variables|Default|GetSocket06)))

(fn IReturnPartReference
  (return 0))