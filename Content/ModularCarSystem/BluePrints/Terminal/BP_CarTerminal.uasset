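; BP_CarTerminal is a proximity terminal that toggles a car info widget for pawns entering or leaving its Sphere.
; Begin overlap acts only while no part is cached: it stores the first BP_MasterCarPart found in the level, then calls APIToogleCarInfoWidget on the pawn controller's BPC_ModularCar.
; End overlap makes the same toggle call every time, and the cached reference is never cleared, so later entries skip the toggle.
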(event OnComponentBeginOverlap(Sphere)
  (params (OverlappedComponent :type Primitive%20Component%20Object%20Reference) (OtherActor :type Actor%20Object%20Reference) (OtherComp :type Primitive%20Component%20Object%20Reference) (OtherBodyIndex :type Integer) (bFromSweep :type Boolean) (SweepResult :type Hit%20Result%20Structure%20%28by%20ref%29))
  (Utilities|IsValid (Variables|Settings|GetMasterModularPartRef)
    (:Is%20Not%20Valid
      (bind _returnvalue (Actor|GetActorOfClass "/Game/ModularCarSystem/BluePrints/CarPart/BP_MasterCarPart.BP_MasterCarPart_C"))
      (Variables|Settings|SetMasterModularPartRef _returnvalue)
      (bind _aspawn (Utilities|Casting|CastToPawn OtherActor))
      (Utilities|IsValid (Actor|GetComponentbyClass (Pawn|GetController _aspawn) "/Game/ModularCarSystem/Component/BPC_ModularCar.BPC_ModularCar_C")
        (:Is%20Valid
          (Default|APIToogleCarInfoWidget (Actor|GetComponentbyClass (Pawn|GetController _aspawn) "/Game/ModularCarSystem/Component/BPC_ModularCar.BPC_ModularCar_C") (Variables|Settings|GetMasterModularPartRef)))))))

(event OnComponentEndOverlap(Sphere)
  (params (OverlappedComponent :type Primitive%20Component%20Object%20Reference) (OtherActor :type Actor%20Object%20Reference) (OtherComp :type Primitive%20Component%20Object%20Reference) (OtherBodyIndex :type Integer))
  (bind _aspawn (Utilities|Casting|CastToPawn OtherActor))
  (Utilities|IsValid (Actor|GetComponentbyClass (Pawn|GetController _aspawn) "/Game/ModularCarSystem/Component/BPC_ModularCar.BPC_ModularCar_C")
    (:Is%20Valid
      (Default|APIToogleCarInfoWidget (Actor|GetComponentbyClass (Pawn|GetController _aspawn) "/Game/ModularCarSystem/Component/BPC_ModularCar.BPC_ModularCar_C") (Variables|Settings|GetMasterModularPartRef)))))

(event EventBeginPlay)

(event Collision|EventActorBeginOverlap
  (params (OtherActor :type Actor%20Object%20Reference)))

(event EventTick
  (params (DeltaSeconds :type Float%20%28single-precision%29)))

(fn ConstructionScript)