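; Base Blueprint for parts in the modular car system, providing shared state and collision handling for building cars from socketed pieces.
; API events forward preview, not-allowed, delete and placed states to empty functions, apparently meant for child overrides.
; Helpers toggle mesh collision for dragging and interaction, and socket sphere collision for snap targeting.
; Sockets are child actors reached through interface calls, which also assign their master part; the part returns itself through an interface.
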(event Custom|API_PartInPreviewMode
  ;[0.15 0.15 0.15 0.5] Handle states
  (States|InPreviewMode))

(event Custom|API_PreviewModeNotAllowed
  ;[0.15 0.15 0.15 0.5] Handle states
  (States|PreviewModeNotAllowed))

(event Custom|API_PartInDeleteMode
  ;[0.15 0.15 0.15 0.5] Handle states
  (States|DeleteMode))

(event Custom|API_PartInPlacedMode
  (params (PlacedSocketRef :type BP%20Base%20Socket%20Object%20Reference))
  ;[0.15 0.15 0.15 0.5] Handle states
  (States|PlacedMode PlacedSocketRef))

(event Custom|API_SetSocketMasterPartRef
  (params (SocketChildMode :type Child%20Actor%20Component%20Object%20Reference) (MasterPartRef :type BP%20Master%20Car%20Part%20Object%20Reference))
  ;[0.15 0.15 0.15 0.5] Set the socket master part reference
  (bind _socket (Class|BPIBaseSocket|IReturnSocketRef(Message) (Variables|/Script/Engine.ChildActorComponent|GetChildActor SocketChildMode)))
  (Variables|/Game/ModularCarSystem/BluePrints/Sockets/BP_BaseSocket.BP_BaseSocket_C|SetMasterPartRef _socket MasterPartRef))

(event EventBeginPlay)

(event Collision|EventActorBeginOverlap
  (params (OtherActor :type Actor%20Object%20Reference)))

(event EventTick
  (params (DeltaSeconds :type Float%20%28single-precision%29)))

(event Custom|API_EnablePartCollision
  (params (Component :type Primitive%20Component%20Object%20Reference))
  ;[0.15 0 0.1035 0.5] This can enable multiple meshes collision so the player can interact with it
  (Collision|SetCollisionResponsetoChannel Component "ECC_Visibility" "ECR_Block")
  (Collision|SetCollisionResponsetoChannel Component "ECC_Camera" "ECR_Block")
  (Collision|SetCollisionResponsetoChannel Component "ECC_Pawn" "ECR_Block"))

(event Custom|API_EnableSocketCollision
  (params (SocketRef :type Child%20Actor%20Component%20Object%20Reference))
  ;[0.15 0.1182 0 0.5] This will enable the socket so the player can target and snap parts on it
  (bind _socket (Class|BPIBaseSocket|IReturnSocketRef(Message) (Variables|/Script/Engine.ChildActorComponent|GetChildActor SocketRef)))
  (Collision|SetCollisionResponsetoChannel (Variables|/Game/ModularCarSystem/BluePrints/Sockets/BP_BaseSocket.BP_BaseSocket_C|GetSphere _socket) "ECC_Visibility" "ECR_Block")
  (Collision|SetCollisionResponsetoChannel (Variables|/Game/ModularCarSystem/BluePrints/Sockets/BP_BaseSocket.BP_BaseSocket_C|GetSphere _socket) "ECC_Camera" "ECR_Ignore")
  (Collision|SetCollisionResponsetoChannel (Variables|/Game/ModularCarSystem/BluePrints/Sockets/BP_BaseSocket.BP_BaseSocket_C|GetSphere _socket) "ECC_Pawn" "ECR_Ignore"))

(event Custom|API_DisableSocketCollision
  (params (Component :type Child%20Actor%20Component%20Object%20Reference))
  ;[0.15 0 0 0.5] Disable the socket collison
  (bind _socket (Class|BPIBaseSocket|IReturnSocketRef(Message) (Variables|/Script/Engine.ChildActorComponent|GetChildActor Component)))
  (Collision|SetCollisionResponsetoChannel (Variables|/Game/ModularCarSystem/BluePrints/Sockets/BP_BaseSocket.BP_BaseSocket_C|GetSphere _socket) "ECC_Visibility" "ECR_Ignore")
  (Collision|SetCollisionResponsetoChannel (Variables|/Game/ModularCarSystem/BluePrints/Sockets/BP_BaseSocket.BP_BaseSocket_C|GetSphere _socket) "ECC_Camera" "ECR_Ignore")
  (Collision|SetCollisionResponsetoChannel (Variables|/Game/ModularCarSystem/BluePrints/Sockets/BP_BaseSocket.BP_BaseSocket_C|GetSphere _socket) "ECC_Pawn" "ECR_Ignore"))

(event Custom|API_DisablePartCollision
  (params (Component :type Primitive%20Component%20Object%20Reference))
  ;[0.15 0 0 0.5] This will disable the mesh collison so we can drag n drop the part around
  (Collision|SetCollisionResponsetoChannel Component "ECC_Visibility" "ECR_Ignore")
  (Collision|SetCollisionResponsetoChannel Component "ECC_Camera" "ECR_Ignore")
  (Collision|SetCollisionResponsetoChannel Component "ECC_Pawn" "ECR_Ignore"))

(fn ConstructionScript)

(fn InPreviewMode)

(fn PlacedMode
  (params (SocketRef :type BP%20Base%20Socket%20Object%20Reference)))

(fn DeleteMode)

(fn PreviewModeNotAllowed)

(fn IReturnPartReference
  (return self))